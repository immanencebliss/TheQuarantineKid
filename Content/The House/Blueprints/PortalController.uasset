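; Controller for the house's portal-order puzzle, armed when the player enters its sphere after at least two puzzles are completed.
; A polled five-second crouch "prayer" closes doors, enables tagged blockers and spawns the first portals.
; Correct portals advance an index driving portal spawns, despawns and door destination swaps; wrong ones tear down the puzzle for retry.
; Finishing the sequence opens FinalPortal, which reports completion to the game mode and spawns the final grimoire.
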(event OnComponentBeginOverlap(Sphere)
  (params (OverlappedComponent :type Primitive%20Component%20Object%20Reference) (OtherActor :type Actor%20Object%20Reference) (OtherComp :type Primitive%20Component%20Object%20Reference) (OtherBodyIndex :type Integer) (bFromSweep :type Boolean) (SweepResult :type Hit%20Result%20Structure%20%28by%20ref%29))
  (if (== OtherActor (Game|GetPlayerCharacter 0))
    (if (>= (Variables|/Game/ThirdPersonBP/Blueprints/ThirdPersonGameMode.ThirdPersonGameMode_C|GetPuzzlesCompleted (.AsThird%20Person%20Game%20Mode (Utilities|Casting|CastToThirdPersonGameMode (Game|GetGameMode)))) 2)
      (if (not (Variables|Default|GetInitialized?))
        (if (Variables|Default|GetCanInitialize?)
          (bind _returnvalue (Utilities|Time|SetTimerbyEvent (delegate Custom|CheckCrouch) 0.1 true))
          (Variables|Default|SetCrouchCheck _returnvalue))))))

(event Custom|Attempt%20Portal
  (params (AttemptedPortal :type BP%20Portal%20Object%20Reference))
  (bind _finalportal (Variables|Default|GetFinalPortal))
  (bind _finalportal_2 (Variables|Default|GetFinalPortal))
  (bind _finalportal_3 (Variables|Default|GetFinalPortal))
  (if (== AttemptedPortal (Variables|Default|GetFinalPortal))
    (for _array_element (Variables|Default|GetPortalSequence)
      (Default|RemovefromPlay _array_element))
    (for _array_element_2 (Variables|Default|GetAdditionalPortals)
      (Default|RemovefromPlay _array_element_2))
    (bind _outactors (Actor|GetAllActorsOfClass "/Game/BlockDoor.BlockDoor_C"))
    (for _array_element_3 _outactors
      (if (Actor|ActorHasTag _array_element_3 "Perpet")
        (Default|Terminate _array_element_3)
        (Utilities|FlowControl|Delay 1.0)
        (Default|Terminate _finalportal_3)
        (Default|Terminate (Variables|/Game/Portals/BP_Portal.BP_Portal_C|GetTargetPortal _finalportal_3))
        (CallFunction|CompletePortalPuzzle)))
    (else
      (bind _newindex (CallFunction|CheckPortal AttemptedPortal (Utilities|Array|Get(acopy) (Variables|Default|GetPortalSequence) (Variables|Default|GetCurrentIndex)) (Variables|Default|GetCurrentIndex)))
      (bind _output_get (Variables|Default|SetCurrentIndex _newindex))
      (if (== _output_get 0)
        (for _array_element_4 (Variables|Default|GetPortalSequence)
          (Default|RemovefromPlay _array_element_4))
        (for _array_element_5 (Variables|Default|GetAdditionalPortals)
          (Default|RemovefromPlay _array_element_5))
        (bind _outactors_2 (Actor|GetAllActorsOfClass "/Game/BlockDoor.BlockDoor_C"))
        (for _array_element_6 _outactors_2
          (if (Actor|ActorHasTag _array_element_6 "Perpet")
            (Default|Terminate _array_element_6)
            (Utilities|FlowControl|Delay 0.5)
            (Default|Terminate _finalportal)
            (Default|Terminate (Variables|/Game/Portals/BP_Portal.BP_Portal_C|GetTargetPortal _finalportal))
            (Variables|Default|SetInitialized? false)))
        (else
          (Default|Terminate AttemptedPortal)
          (Default|ReplacewithStatic AttemptedPortal)
          (Utilities|FlowControl|Sequence
            (:then_0
              (if (>= _output_get (Utilities|Array|Length (Variables|Default|GetPortalSequence)))
                (Default|Initialize _finalportal_2)
                (Default|Initialize (Variables|/Game/Portals/BP_Portal.BP_Portal_C|GetTargetPortal _finalportal_2))))
            (:then_1
              (Utilities|FlowControl|Delay 0.5)
              (Default|ReplacewithStatic (Variables|/Game/Portals/BP_Portal.BP_Portal_C|GetTargetPortal AttemptedPortal))
              (for _array_element_7 (Variables|Default|GetPortalSequence)
                (if (== (Variables|/Game/Portals/BP_Portal.BP_Portal_C|GetSpawnIndex _array_element_7) (Variables|Default|GetCurrentIndex))
                  (Default|Initialize _array_element_7)))
              (for _array_element_8 (Variables|Default|GetAdditionalPortals)
                (if (== (Variables|/Game/Portals/BP_Portal.BP_Portal_C|GetSpawnIndex _array_element_8) (Variables|Default|GetCurrentIndex))
                  (Default|Initialize _array_element_8)))
              (bind _outactors_3 (Actor|GetAllActorsOfClass "/Game/HQ_ResidentialHouse/Actors/BP_DoorWide.BP_DoorWide_C"))
              (for _array_element_9 _outactors_3
                (if (== (Variables|/Game/HQ_ResidentialHouse/Actors/BP_DoorWide.BP_DoorWide_C|GetDestinationSwapIndex _array_element_9) (Variables|Default|GetCurrentIndex))
                  (Default|SwapDestination _array_element_9)))
              (for _array_element_10 (Variables|Default|GetPortalSequence)
                (if (== (Variables|/Game/Portals/BP_Portal.BP_Portal_C|GetDespawnIndex _array_element_10) (Variables|Default|GetCurrentIndex))
                  (Default|Terminate _array_element_10)))
              (for _array_element_11 (Variables|Default|GetAdditionalPortals)
                (if (== (Variables|/Game/Portals/BP_Portal.BP_Portal_C|GetDespawnIndex _array_element_11) (Variables|Default|GetCurrentIndex))
                  (Default|Terminate _array_element_11))))))))))

(event Custom|CheckCrouch
  (bind _asfirst_person_character (Utilities|Casting|CastToFirstPersonCharacter (Game|GetPlayerCharacter 0)))
  (if (Variables|/Game/FirstPersonBP/Blueprints/FirstPersonCharacter.FirstPersonCharacter_C|GetCrouching _asfirst_person_character)
    (Utilities|FlowControl|DoOnce false :!label _label
      (:Completed
        (bind _returnvalue (Utilities|Time|SetTimerbyEvent (delegate Custom|PrayerComplete) 5.0))))
    (else
      (Utilities|Time|ClearandInvalidateTimerbyHandle _returnvalue)
      (goto _label Reset))))

(event Custom|PrayerComplete
  (Utilities|Time|ClearandInvalidateTimerbyHandle (Variables|Default|GetCrouchCheck))
  (bind _outactors (Actor|GetAllActorsOfClass "/Game/HQ_ResidentialHouse/Actors/BP_DoorWide.BP_DoorWide_C"))
  (for _array_element _outactors
    (Default|ForceClosed _array_element)
    (for _array_element_2 (Variables|Default|GetPortalSequence)
      (if (== (Variables|/Game/Portals/BP_Portal.BP_Portal_C|GetSpawnIndex _array_element_2) 0)
        (Default|Initialize _array_element_2)))
    (for _array_element_3 (Variables|Default|GetAdditionalPortals)
      (if (== (Variables|/Game/Portals/BP_Portal.BP_Portal_C|GetSpawnIndex _array_element_3) 0)
        (Default|Initialize _array_element_3)))
    (bind _outactors_2 (Actor|GetAllActorsOfClass "/Game/BlockDoor.BlockDoor_C"))
    (for _array_element_4 _outactors_2
      (if (Actor|ActorHasTag _array_element_4 "Perpet")
        (Default|Enable _array_element_4)))
    (Variables|Default|SetInitialized? true)
    (Variables|/Game/FirstPersonBP/Blueprints/FirstPersonCharacter.FirstPersonCharacter_C|SetPortalController (.AsFirst%20Person%20Character (Utilities|Casting|CastToFirstPersonCharacter (Game|GetPlayerCharacter 0))) self)))

(event Custom|CompletePortalPuzzle
  (bind _returnvalue (Game|GetGameMode))
  (bind _asthird_person_game_mode (Utilities|Casting|CastToThirdPersonGameMode _returnvalue))
  (Variables|Default|SetCanInitialize? false)
  (Variables|/Game/ThirdPersonBP/Blueprints/ThirdPersonGameMode.ThirdPersonGameMode_C|SetPortalPuzzleComplete _asthird_person_game_mode true)
  (Default|SpawnFinalGrimoire _asthird_person_game_mode)
  (Default|LightUpCircle _asthird_person_game_mode (Variables|Default|GetPuzzleType))
  (Math|Integer|IncrementInt (Variables|/Game/ThirdPersonBP/Blueprints/ThirdPersonGameMode.ThirdPersonGameMode_C|GetPuzzlesCompleted _asthird_person_game_mode)))

(fn ConstructionScript)

(fn CheckPortal
  (params (Attempted%20Portal :type BP%20Portal%20Object%20Reference) (Correct%20Portal :type BP%20Portal%20Object%20Reference) (CurrentIndex :type Integer))
  (bind _output_get (LocalVariables|SetLocalIndex CurrentIndex))
  (if (== Attempted%20Portal Correct%20Portal)
    (bind _result (Math|Integer|IncrementInt _output_get)
      (:%20%20
        (return _result)))
    (else
      (return 0))))