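; BP_LowerBTSpookTrigger is the trigger that runs the lower bathroom scare when the player overlaps it during room 3.
; Once only, it registers with the cell phone widget, locks door and light switch, then sequences flickering lights, texts, window banging and the BasementDweller's entrance and dissolve using delays.
; Interact and ResetEnviornment share a path that unlocks the switch and forces the door.
; SpookTrigger hands off to FinaleControl to start the finale.
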(event OnComponentBeginOverlap(Spooker)
  (params (OverlappedComponent :type Primitive%20Component%20Object%20Reference) (OtherActor :type Actor%20Object%20Reference) (OtherComp :type Primitive%20Component%20Object%20Reference) (OtherBodyIndex :type Integer) (bFromSweep :type Boolean) (SweepResult :type Hit%20Result%20Structure%20%28by%20ref%29))
  (bind _basementdweller (Variables|Default|GetBasementDweller))
  (bind _door (Variables|Default|GetDoor))
  (if (and (Actor|ActorHasTag OtherActor "player") (== (Variables|/Game/ThirdPersonBP/Blueprints/ThirdPersonGameMode.ThirdPersonGameMode_C|GetCurrentRoomToMark (.AsThird%20Person%20Game%20Mode (Utilities|Casting|CastToThirdPersonGameMode (Game|GetGameMode)))) 3))
    (Utilities|FlowControl|DoOnce false
      (:Completed
        (bind _foundwidgets (Widget|GetAllWidgetsOfClass "/Game/Blueprints/Cellphone/WID_CellPhoneMaster.WID_CellPhoneMaster_C" false))
        (Variables|/Game/Blueprints/Cellphone/WID_CellPhoneMaster.WID_CellPhoneMaster_C|SetSpookTrigger (Utilities|Array|Get(acopy) _foundwidgets) self)
        (Utilities|FlowControl|Delay 1.0)
        (Default|SlamDoor _door)
        (Variables|/Game/HQ_ResidentialHouse/Actors/BP_DoorWide.BP_DoorWide_C|SetdoorLocked _door true)
        (Variables|/Game/LightSwitch.LightSwitch_C|SetisLocked (Variables|Default|GetLightSwitch) true)
        (for _array_element (Variables|Default|GetLights)
          (Class|LightInterface|IFlickeron(Message) _array_element false)
          (Utilities|FlowControl|Delay 1.0)
          (bind _foundwidgets_2 (Widget|GetAllWidgetsOfClass "/Game/Blueprints/Cellphone/WID_CellPhoneMaster.WID_CellPhoneMaster_C" false))
          (Default|BathroomTexts (Utilities|Array|Get(acopy) _foundwidgets_2))
          (Default|PlaySound (Variables|Default|GetWindowBaning))
          (Utilities|FlowControl|Delay 4.0)
          (Rendering|SetVisibility (Variables|/Script/Engine.SkeletalMeshActor|GetSkeletalMeshComponent _basementdweller) true false)
          (Default|Walkin _basementdweller)
          (Utilities|FlowControl|Delay 1.0)
          (for _array_element_2 (Variables|Default|GetLights)
            (Class|LightInterface|IFlickerOff(Message) _array_element_2 false))
          (Utilities|FlowControl|Delay 7.0)
          (Default|DissolveDweller _basementdweller))))))

(event Custom|ResetEnviornment
  (bind _door (Variables|Default|GetDoor))
  (Utilities|FlowControl|Delay 1.0)
  (for _array_element (Variables|Default|GetLights)
    (Class|LightInterface|IFlickerShort(Message) _array_element false)
    (Variables|/Game/LightSwitch.LightSwitch_C|SetisLocked (Variables|Default|GetLightSwitch) false))
  (Utilities|FlowControl|Delay 1.5)
  (Variables|/Game/HQ_ResidentialHouse/Actors/BP_DoorWide.BP_DoorWide_C|SetdoorLocked _door false)
  (Default|Force _door))

(event EventInteract
  (params (HitComponent :type Actor%20Component%20Object%20Reference))
  (bind _door (Variables|Default|GetDoor))
  (Utilities|FlowControl|Delay 1.0)
  (for _array_element (Variables|Default|GetLights)
    (Class|LightInterface|IFlickerShort(Message) _array_element false)
    (Variables|/Game/LightSwitch.LightSwitch_C|SetisLocked (Variables|Default|GetLightSwitch) false))
  (Utilities|FlowControl|Delay 1.5)
  (Variables|/Game/HQ_ResidentialHouse/Actors/BP_DoorWide.BP_DoorWide_C|SetdoorLocked _door false)
  (Default|Force _door))

(event EventSpookTrigger
  (Default|InitiateFinale (Variables|Default|GetFinaleControl)))

(fn ConstructionScript)