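; Ritual circle in the chapel that the player completes by passing its points in sequence, starting from any point.
; CirclePointCheck tracks the expected point, raising the dynamic material's brightness and visibility through a timeline on each correct step and resetting on a wrong one.
; Completion eases the glow down, calls ChapelCheck on ThirdPersonGameMode and spawns grimoire pages according to the Candle and Moonlight flags.
; Detail-circle logic is left unwired.
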(event Custom|CircleMatieralTimeLine
  (bind _basecircle (Timeline|CircleVisibility Play)
    (:Update
      (Rendering|Material|SetScalarParameterValue (Variables|Default|GetBaseCircleMat) "Brightness" (Math|Float|Lerp (Variables|LerpValues|GetCurrentPositionBrightness) (Variables|LerpValues|GetTargetPositionBrightness) _basecircle) :!class /Script/Engine.MaterialInstanceDynamic)
      (Rendering|Material|SetScalarParameterValue (Variables|Default|GetBaseCircleMat) "Visibility" (Math|Float|Lerp (Variables|LerpValues|GetCurrentPositionVisibility) (Variables|LerpValues|GetTargetPositionvisibility) _basecircle) :!class /Script/Engine.MaterialInstanceDynamic))
    (:Finished
      (CallFunction|SetCurrentVisandBright))))

(event Custom|DetailCircleTimeLine
  (bind _detaillerp (Timeline|DetailCircleVisibility Play)
    (:Finished
      (CallFunction|SetCurrentVisandBrightDetail))))

(event Custom|UnGlow
  (bind _eccentricitylerp (Timeline|SuperCircleFlash Play)
    (:Update
      (Rendering|Material|SetScalarParameterValue (Variables|Default|GetBaseCircleMat) "Brightness" (Math|Float|Lerp 6.0 (Variables|Default|GetnormalGlow) _eccentricitylerp) :!class /Script/Engine.MaterialInstanceDynamic))))

(event Collision|EventActorBeginOverlap
  (params (OtherActor :type Actor%20Object%20Reference)))

(event EventTick
  (params (DeltaSeconds :type Float%20%28single-precision%29)))

(event EventBeginPlay
  (Rendering|SetVisibility (Variables|Default|GetBaseCircle) false false)
  (CallFunction|CalculateLerpAmounts)
  (Rendering|Material|SetScalarParameterValue (Variables|Default|GetBaseCircleMat) "Brightness" 0.0 :!class /Script/Engine.MaterialInstanceDynamic)
  (Rendering|Material|SetScalarParameterValue (Variables|Default|GetBaseCircleMat) "Visibility" 0.0 :!class /Script/Engine.MaterialInstanceDynamic))

(fn ConstructionScript
  (bind _returnvalue (Rendering|Material|CreateDynamicMaterialInstance (Variables|Default|GetBaseCircle) 0 "/Game/Blueprints/RitualBps/CircleWalk/MATINST_RitualCircleBase.MATINST_RitualCircleBase" "None" :!class /Script/Engine.PrimitiveComponent))
  (bind _output_get (Variables|Default|SetBaseCircleMat _returnvalue))
  (Rendering|Material|SetTextureParameterValue _output_get "circle" (Variables|Default|GetMagicCircle)))

(fn CirclePointCheck
  (params (CirclePoint :type Integer))
  (bind _defaultsceneroot (Variables|Default|GetDefaultSceneRoot))
  (bind _defaultsceneroot_2 (Variables|Default|GetDefaultSceneRoot))
  (bind _returnvalue (Transformation|GetWorldLocation _defaultsceneroot))
  (bind _returnvalue_2 (Transformation|GetWorldLocation _defaultsceneroot_2))
  (bind (_x _y _z) (Math|Vector|BreakVector _returnvalue_2))
  (bind (_x_2 _y_2 _z_2) (Math|Vector|BreakVector _returnvalue))
  (if (not (Variables|Default|GetFinished?))
    (Variables|Default|SetCurrentCirclePoint CirclePoint)
    (if (Variables|Default|GetCircleStarted?)
      (if (== (Variables|Default|GetCurrentCirclePoint) (Variables|Default|GetExpectedCirclePoint))
        (Math|Integer|IncrementInt (Variables|Default|GetExpectedCirclePoint)
          (:%20%20
            (if (> (Variables|Default|GetExpectedCirclePoint) (- (Math|Float|Truncate (Variables|Default|GetTotalCirclePoints)) 1))
              (Variables|Default|SetExpectedCirclePoint 1))
            (if (>= (Variables|Default|GetNumber%20Of%20Circle%20Points%20Passed) (Math|Float|Truncate (Variables|Default|GetTotalCirclePoints)))
              (Variables|Default|SetFinished? true)
              (CallFunction|UnGlow)
              (bind _asthird_person_game_mode (Utilities|Casting|CastToThirdPersonGameMode (Game|GetGameMode)))
              (Default|ChapelCheck _asthird_person_game_mode)
              (Utilities|FlowControl|Sequence
                (:then_0
                  (if (Variables|Default|GetCandle)
                    (bind _returnvalue_3 (Game|SpawnActorfromClass "/Game/Blueprints/RitualBps/BPGrimoirePage.BPGrimoirePage_C" (Math|Conversions|ToTransform(Vector) (Math|Vector|MakeVector _x _y (+ _z 1.0))) "Undefined" 0 0))
                    (Default|SetPage _returnvalue_3 false)))
                (:then_1
                  (if (Variables|Default|GetMoonlight)
                    (bind _returnvalue_4 (Game|SpawnActorfromClass "/Game/Blueprints/RitualBps/BPGrimoirePage.BPGrimoirePage_C" (Math|Conversions|ToTransform(Vector) (Math|Vector|MakeVector _x_2 _y_2 (+ _z_2 1.0))) "Undefined" 0 0))
                    (Default|SetPage _returnvalue_4 true 1))))
              (else
                (Math|Integer|IncrementInt (Variables|Default|GetNumber%20Of%20Circle%20Points%20Passed)
                  (:%20%20
                    (Variables|LerpValues|SetTargetPositionBrightness (+ (Variables|LerpValues|GetTargetPositionBrightness) (Variables|LerpValues|GetBrightnessToAdd)))
                    (Variables|LerpValues|SetTargetPositionvisibility (+ (Variables|LerpValues|GetTargetPositionvisibility) (Variables|LerpValues|GetVisibilityToAdd)))
                    (CallFunction|CircleMatieralTimeLine)))))))
        (else
          (CallFunction|Resetcircle)))
      (else
        (bind _result (Math|Integer|IncrementInt (Variables|Default|GetCurrentCirclePoint))
          (:%20%20
            (Variables|Default|SetExpectedCirclePoint _result)
            (Math|Integer|IncrementInt (Variables|Default|GetNumber%20Of%20Circle%20Points%20Passed)
              (:%20%20
                (Variables|Default|SetCircleStarted? true)
                (Rendering|SetVisibility (Variables|Default|GetBaseCircle) true false)))))))))

(fn CalculateLerpAmounts
  (bind _totalcirclepoints (Variables|Default|GetTotalCirclePoints))
  (bind _returnvalue (- _totalcirclepoints 1.0))
  (bind _returnvalue_2 (- _totalcirclepoints 4.0))
  (Utilities|FlowControl|Sequence
    (:then_0
      (Variables|LerpValues|SetBrightnessToAdd (/ 6.0 _returnvalue))
      (Variables|LerpValues|SetVisibilityToAdd (/ 1.0 _returnvalue))
      (Variables|LerpValuesDetail|SetBrightnessToAddDetail (/ 6.0 _returnvalue_2))
      (Variables|LerpValuesDetail|SetVisibilityToDetail (/ 1.0 _returnvalue_2)))))

(fn SetCurrentVisandBright
  (Variables|LerpValues|SetCurrentPositionBrightness (+ (Variables|LerpValues|GetCurrentPositionBrightness) (Variables|LerpValues|GetBrightnessToAdd)))
  (Variables|LerpValues|SetCurrentPositionVisibility (+ (Variables|LerpValues|GetCurrentPositionVisibility) (Variables|LerpValues|GetVisibilityToAdd))))

(fn Resetcircle
  (Utilities|FlowControl|Sequence
    (:then_0
      (Variables|Default|SetCircleStarted? false)
      (Variables|Default|SetNumber%20Of%20Circle%20Points%20Passed 0))
    (:then_1
      (Variables|LerpValues|SetCurrentPositionBrightness 0.0)
      (Variables|LerpValues|SetTargetPositionBrightness (Variables|LerpValues|GetBrightnessToAdd))
      (Variables|LerpValues|SetCurrentPositionVisibility 0.0)
      (Variables|LerpValues|SetTargetPositionvisibility (Variables|LerpValues|GetVisibilityToAdd)))
    (:then_2
      (Rendering|SetVisibility (Variables|Default|GetBaseCircle) false false)
      (Rendering|Material|SetScalarParameterValue (Variables|Default|GetBaseCircleMat) "Brightness" 0.0 :!class /Script/Engine.MaterialInstanceDynamic)
      (Rendering|Material|SetScalarParameterValue (Variables|Default|GetBaseCircleMat) "Visibility" 0.0 :!class /Script/Engine.MaterialInstanceDynamic))))

(fn SetCurrentVisandBrightDetail
  (Variables|LerpValuesDetail|SetCurrentPositionBrightnessDetail (+ (Variables|LerpValuesDetail|GetCurrentPositionBrightnessDetail) (Variables|LerpValuesDetail|GetBrightnessToAddDetail)))
  (Variables|LerpValuesDetail|SetCurrentPositionVisibilityDetail (+ (Variables|LerpValuesDetail|GetCurrentPositionVisibilityDetail) (Variables|LerpValuesDetail|GetVisibilityToDetail))))