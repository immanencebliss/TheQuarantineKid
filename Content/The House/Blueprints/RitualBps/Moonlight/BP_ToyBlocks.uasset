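; Interactable toy block for the Moonlight ritual puzzle, showing one symbol from the M-A-R-I-E set.
; It starts hidden and non-collidable; a one-time interaction fades it out, teleports it to its letter's fixed slot and registers it with BlockMaster.
; Construction sets its color and textures on dynamic materials.
; When BlockMaster is open, a dissolve timeline swaps the symbol between letter and number textures at its faded point via DoOnce.
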(event Custom|Vanish%20Block
  (bind _blockvisibility (Timeline|BlockVanish Play)
    (:Update
      (Rendering|Material|SetScalarParameterValue (Variables|Default|GetBlockMat) "visbility" (Math|Float|Lerp 1.0 0.0 _blockvisibility) :!class /Script/Engine.MaterialInstanceDynamic)
      (Rendering|Material|SetScalarParameterValue (Variables|Default|GetBlockSymbol) "disolve" (Math|Float|Lerp 1.0 0.0 _blockvisibility) :!class /Script/Engine.MaterialInstanceDynamic))
    (:Finished
      (Transformation|SetWorldLocation (Variables|Default|GetDefaultSceneRoot) (Variables|Default|GetTeleportLocation) false false)
      (Rendering|Material|SetScalarParameterValue (Variables|Default|GetBlockMat) "visbility" 1.0 :!class /Script/Engine.MaterialInstanceDynamic)
      (Rendering|Material|SetScalarParameterValue (Variables|Default|GetBlockSymbol) "disolve" 1.0 :!class /Script/Engine.MaterialInstanceDynamic)
      (if (Variables|/Game/Blueprints/RitualBps/Moonlight/BPMoonlightShade.BPMoonlightShade_C|GetOpen (Variables|Default|GetBlockMaster))
        (CallFunction|DisolveSymbol)))))

(event Custom|DisolveSymbol
  (bind _dissolvetrack (Timeline|dissolving PlayFromStart)
    (:Update
      (if (<= (Math|Float|Lerp 1.0 0.0 _dissolvetrack) 0.05)
        (Utilities|FlowControl|DoOnce false
          (:Completed
            (CallFunction|SwitchSymbol))))
      (Rendering|Material|SetScalarParameterValue (Variables|Default|GetBlockSymbol) "disolve" (Math|Float|Lerp 1.0 0.0 _dissolvetrack) :!class /Script/Engine.MaterialInstanceDynamic))
    (:Finished
      (CallFunction|Reset))))

(event Custom|Reset
  (Utilities|FlowControl|DoOnce false) ; enters at Reset
)

(event EventBeginPlay
  (Rendering|Material|SetTextureParameterValue (Variables|Default|GetBlockSymbol) "let" (Variables|Default|GetLetter))
  (Input|EnableInput (Game|GetPlayerController 0))
  (CallFunction|TurnOffBlock))

(event Collision|EventActorBeginOverlap
  (params (OtherActor :type Actor%20Object%20Reference)))

(event EventTick
  (params (DeltaSeconds :type Float%20%28single-precision%29)))

(event EventInteract
  (params (HitComponent :type Actor%20Component%20Object%20Reference))
  (bind _blockmaster (Variables|Default|GetBlockMaster))
  (if (not (Variables|Default|GetDone))
    (switch Utilities|FlowControl|Switch|SwitchonENU_BlockLetter (Variables|Default|GetBlockLetter)
      (:NewEnumerator0
        (Variables|Default|SetTeleportLocation "-392.367523,-304.129944,267.674072"))
      (:NewEnumerator1
        (Variables|Default|SetTeleportLocation "-392.367523,-290.532379,267.674072"))
      (:NewEnumerator2
        (Variables|Default|SetTeleportLocation "-392.367523,-275.567383,267.674072"))
      (:NewEnumerator3
        (Variables|Default|SetTeleportLocation "-392.367523,-261.508057,267.674072"))
      (:NewEnumerator4
        (Variables|Default|SetTeleportLocation "-392.367523,-248.119385,267.674072")))
    (CallFunction|VanishBlock)
    (Utilities|Array|Add (Variables|/Game/Blueprints/RitualBps/Moonlight/BPMoonlightShade.BPMoonlightShade_C|GetBlockinRoom _blockmaster) self)
    (Variables|Default|SetDone true)
    (if (Variables|/Game/Blueprints/RitualBps/Moonlight/BPMoonlightShade.BPMoonlightShade_C|GetOpen _blockmaster)
      (CallFunction|DisolveSymbol))))

(fn ConstructionScript
  (bind _returnvalue (Rendering|Material|CreateDynamicMaterialInstance (Variables|Default|GetKidsBlock) 0 "/Game/Matieral/KidsBlocks/Mat_KidsBlock_Inst.Mat_KidsBlock_Inst" "None" :!class /Script/Engine.PrimitiveComponent))
  (Variables|Default|SetBlockMat _returnvalue)
  (bind _returnvalue_2 (Rendering|Material|CreateDynamicMaterialInstance (Variables|Default|GetPlane) 0 "/Game/Matieral/KidsBlocks/Mat_BlockSymbol_Inst.Mat_BlockSymbol_Inst" "let" :!class /Script/Engine.PrimitiveComponent))
  (Variables|Default|SetBlockSymbol _returnvalue_2)
  (CallFunction|SetSymbolsandColor))

(fn SetSymbolsandColor
  (switch Utilities|FlowControl|Switch|SwitchonENU_BlockLetter (Variables|Default|GetBlockLetter)
    (:NewEnumerator0
      (Variables|Default|SetSymbolIndex 0))
    (:NewEnumerator1
      (Variables|Default|SetSymbolIndex 1))
    (:NewEnumerator2
      (Variables|Default|SetSymbolIndex 2))
    (:NewEnumerator3
      (Variables|Default|SetSymbolIndex 3))
    (:NewEnumerator4
      (Variables|Default|SetSymbolIndex 4)))
  (Utilities|SetTextures (Utilities|Array|Get(acopy) (Variables|Default|GetLETTERS) (Variables|Default|GetSymbolIndex)) (Utilities|Array|Get(acopy) (Variables|Default|GetNUMBERS) (Variables|Default|GetSymbolIndex))
    (:%20
      (Rendering|Material|SetTextureParameterValue (Variables|Default|GetBlockSymbol) "let" (Variables|Default|GetLetter))
      (Rendering|Material|SetVectorParameterValue (Variables|Default|GetBlockMat) "color" (Variables|Default|GetColor) :!class /Script/Engine.MaterialInstanceDynamic))))

(fn SwitchSymbol
  (if (Variables|Default|GetisinMoonlight?)
    (Variables|Default|SetisinMoonlight? false)
    (Rendering|Material|SetTextureParameterValue (Variables|Default|GetBlockSymbol) "let" (Variables|Default|GetNumber))
    (else
      (Variables|Default|SetisinMoonlight? true)
      (Rendering|Material|SetTextureParameterValue (Variables|Default|GetBlockSymbol) "let" (Variables|Default|GetLetter)))))

(fn TurnonBlock
  (bind _kidsblock (Variables|Default|GetKidsBlock))
  (Rendering|SetVisibility _kidsblock true false)
  (Collision|SetCollisionEnabled _kidsblock "QueryAndPhysics"))

(fn TurnOffBlock
  (bind _kidsblock (Variables|Default|GetKidsBlock))
  (Rendering|SetVisibility _kidsblock false false)
  (Collision|SetCollisionEnabled _kidsblock "NoCollision"))