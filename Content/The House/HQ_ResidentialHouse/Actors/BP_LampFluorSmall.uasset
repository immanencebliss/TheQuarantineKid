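; Small fluorescent lamp actor that can be toggled, flickered and visibility-culled through events, including monster cull variants.
; Construction caches rect lights, their default intensity and a dynamic glass material, then applies the IsOff state.
; Toggle sets lights and emission together; long, short and looping flickers lerp both via timelines, played forward or reversed.
; Short and looping flickers use a Points array, which construction never fills, instead of Rects.
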(event Custom|CustomEvent_2
  (params (FlickerOn? :type Boolean))
  ;[1 1 1] Flicker lights Looping
  (bind _output_get (Variables|Default|SetFlickOn FlickerOn?))
  (if _output_get
    (bind _newtrack_0 (Timeline|Timeline_3 ReverseFromEnd)
      (:Update
        (for _array_element (Variables|Default|GetPoints)
          (Rendering|Components|Light|SetIntensity _array_element (Math|Float|Lerp 0.0 (Variables|Default|GetDefault%20Intensity) _newtrack_0))
          (if (Variables|Default|GetFlickOn)
            (Rendering|SetVisibility _array_element true true)
            (Rendering|Material|SetScalarParameterValue (Variables|Default|GetMatInstance) "Emission Intensity" (Math|Float|Lerp 0.0 15.0 _newtrack_0) :!class /Script/Engine.MaterialInstanceDynamic)
            (Variables|Default|SetIsOff? false)
            (else
              (Rendering|SetVisibility _array_element true true)
              (Rendering|Material|SetScalarParameterValue (Variables|Default|GetMatInstance) "Emission Intensity" (Math|Float|Lerp 0.0 15.0 _newtrack_0) :!class /Script/Engine.MaterialInstanceDynamic)
              (Variables|Default|SetIsOff? true))))))
    (else
      (Timeline|Timeline_3 PlayFromStart))))

(event Custom|Flicker%20Lights%20Long
  (params (FlickerOn? :type Boolean))
  ;[1 1 1] Flicker lights long
  (bind _output_get (Variables|Default|SetFlickOn FlickerOn?))
  (if _output_get
    (bind _newtrack_0 (Timeline|Timeline_1_0 ReverseFromEnd)
      (:Update
        (for _array_element (Variables|Default|GetRects)
          (Rendering|Components|Light|SetIntensity _array_element (Math|Float|Lerp 0.0 (Variables|Default|GetDefault%20Intensity) _newtrack_0))
          (if (Variables|Default|GetFlickOn)
            (Rendering|SetVisibility _array_element true true)
            (Rendering|Material|SetScalarParameterValue (Variables|Default|GetMatInstance) "Emission Intensity" (Math|Float|Lerp 0.0 15.0 _newtrack_0) :!class /Script/Engine.MaterialInstanceDynamic)
            (Variables|Default|SetIsOff? false)
            (else
              (Rendering|SetVisibility _array_element true true)
              (Rendering|Material|SetScalarParameterValue (Variables|Default|GetMatInstance) "Emission Intensity" (Math|Float|Lerp 0.0 15.0 _newtrack_0) :!class /Script/Engine.MaterialInstanceDynamic)
              (Variables|Default|SetIsOff? true))))))
    (else
      (Timeline|Timeline_1_0 PlayFromStart))))

(event Custom|CustomEvent_1
  (params (FlickerOn? :type Boolean))
  ;[1 1 1] Flicker lights Short
  (bind _output_get (Variables|Default|SetFlickOn FlickerOn?))
  (if _output_get
    (bind _newtrack_0 (Timeline|Timeline_2_0 ReverseFromEnd)
      (:Update
        (for _array_element (Variables|Default|GetPoints)
          (Rendering|Components|Light|SetIntensity _array_element (Math|Float|Lerp 0.0 (Variables|Default|GetDefault%20Intensity) _newtrack_0))
          (if (Variables|Default|GetFlickOn)
            (Rendering|SetVisibility _array_element true true)
            (Rendering|Material|SetScalarParameterValue (Variables|Default|GetMatInstance) "Emission Intensity" (Math|Float|Lerp 0.0 15.0 _newtrack_0) :!class /Script/Engine.MaterialInstanceDynamic)
            (Variables|Default|SetIsOff? false)
            (else
              (Rendering|SetVisibility _array_element true true)
              (Rendering|Material|SetScalarParameterValue (Variables|Default|GetMatInstance) "Emission Intensity" (Math|Float|Lerp 0.0 15.0 _newtrack_0) :!class /Script/Engine.MaterialInstanceDynamic)
              (Variables|Default|SetIsOff? true))))))
    (else
      (Timeline|Timeline_2_0 PlayFromStart))))

(event Custom|CustomEvent_3
  (params (Flick%20On :type Boolean))
  ;[1 1 1] Flicker lights Looping
  (Utilities|FlowControl|Sequence
    (:then_0
      (bind _newtrack_0 (Timeline|Timeline_3 Stop)
        (:Update
          (for _array_element (Variables|Default|GetPoints)
            (Rendering|Components|Light|SetIntensity _array_element (Math|Float|Lerp 0.0 (Variables|Default|GetDefault%20Intensity) _newtrack_0))
            (if (Variables|Default|GetFlickOn)
              (Rendering|SetVisibility _array_element true true)
              (Rendering|Material|SetScalarParameterValue (Variables|Default|GetMatInstance) "Emission Intensity" (Math|Float|Lerp 0.0 15.0 _newtrack_0) :!class /Script/Engine.MaterialInstanceDynamic)
              (Variables|Default|SetIsOff? false)
              (else
                (Rendering|SetVisibility _array_element true true)
                (Rendering|Material|SetScalarParameterValue (Variables|Default|GetMatInstance) "Emission Intensity" (Math|Float|Lerp 0.0 15.0 _newtrack_0) :!class /Script/Engine.MaterialInstanceDynamic)
                (Variables|Default|SetIsOff? true)))))))
    (:then_1
      (if Flick%20On
        (for _array_element_2 (Variables|Default|GetPoints)
          (Rendering|Components|Light|SetIntensity _array_element_2 (Variables|Default|GetDefault%20Intensity))
          (if (Variables|Default|GetFlickOn)
            (Rendering|SetVisibility _array_element true true)
            (Rendering|Material|SetScalarParameterValue (Variables|Default|GetMatInstance) "Emission Intensity" (Math|Float|Lerp 0.0 15.0 _newtrack_0) :!class /Script/Engine.MaterialInstanceDynamic)
            (Variables|Default|SetIsOff? false)
            (else
              (Rendering|SetVisibility _array_element true true)
              (Rendering|Material|SetScalarParameterValue (Variables|Default|GetMatInstance) "Emission Intensity" (Math|Float|Lerp 0.0 15.0 _newtrack_0) :!class /Script/Engine.MaterialInstanceDynamic)
              (Variables|Default|SetIsOff? true))))
        (else
          (for _array_element_3 (Variables|Default|GetPoints)
            (Rendering|Components|Light|SetIntensity _array_element_3 0.0)
            (if (Variables|Default|GetFlickOn)
              (Rendering|SetVisibility _array_element true true)
              (Rendering|Material|SetScalarParameterValue (Variables|Default|GetMatInstance) "Emission Intensity" (Math|Float|Lerp 0.0 15.0 _newtrack_0) :!class /Script/Engine.MaterialInstanceDynamic)
              (Variables|Default|SetIsOff? false)
              (else
                (Rendering|SetVisibility _array_element true true)
                (Rendering|Material|SetScalarParameterValue (Variables|Default|GetMatInstance) "Emission Intensity" (Math|Float|Lerp 0.0 15.0 _newtrack_0) :!class /Script/Engine.MaterialInstanceDynamic)
                (Variables|Default|SetIsOff? true)))))))))

(event EventToggleLight
  (params (Off? :type Boolean))
  (bind _rects (Variables|Default|GetRects))
  ;[1 1 1] Toggle Light
  (if (Variables|Default|GetIsOff?)
    (for _array_element _rects
      (Rendering|Components|Light|SetIntensity _array_element (Variables|Default|GetDefault%20Intensity))
      (Rendering|SetVisibility _array_element true false)
      (Variables|Default|SetIsOff? false)
      (Rendering|Material|SetScalarParameterValue (Variables|Default|GetMatInstance) "Emission Intensity" 15.0 :!class /Script/Engine.MaterialInstanceDynamic))
    (else
      (for _array_element_2 _rects
        (Rendering|Components|Light|SetIntensity _array_element_2 0.0)
        (Rendering|SetVisibility _array_element_2 false false)
        (Variables|Default|SetIsOff? true)
        (Rendering|Material|SetScalarParameterValue (Variables|Default|GetMatInstance) "Emission Intensity" 0.0 :!class /Script/Engine.MaterialInstanceDynamic)))))

(event EventCullLighting
  (Rendering|SetVisibility (Variables|Default|GetRectLight) false false))

(event EventMonsterCull
  (Rendering|SetVisibility (Variables|Default|GetRectLight) false false))

(event EventUncullLighting
  (Rendering|SetVisibility (Variables|Default|GetRectLight) true false))

(event EventMonsterUncull
  (Rendering|SetVisibility (Variables|Default|GetRectLight) true false))

(fn ConstructionScript
  (bind _lampfluor_glass (Variables|Default|GetLampFluor_Glass))
  (Utilities|FlowControl|Sequence
    (:then_0
      (bind _output_get (Variables|Default|SetRects (Actor|GetComponentsByClass "/Script/Engine.RectLightComponent")))
      (Variables|Default|SetDefault%20intensity (Variables|/Script/Engine.LightComponentBase|GetIntensity (Utilities|Array|Get(acopy) _output_get))))
    (:then_1
      (bind _returnvalue (Rendering|Material|CreateDynamicMaterialInstance _lampfluor_glass 0 (Rendering|Material|GetMaterial _lampfluor_glass 0) "None" :!class /Script/Engine.PrimitiveComponent))
      (Variables|Default|SetMatInstance _returnvalue)
      (for _array_element (Variables|Default|GetRects)
        (if (Variables|Default|GetIsOff?)
          (Rendering|SetVisibility _array_element false false)
          (Rendering|Material|SetScalarParameterValue (Variables|Default|GetMatInstance) "Emission Intensity" 0.0 :!class /Script/Engine.MaterialInstanceDynamic)
          (else
            (Rendering|SetVisibility _array_element true false)
            (Rendering|Material|SetScalarParameterValue (Variables|Default|GetMatInstance) "Emission Intensity" 15.0 :!class /Script/Engine.MaterialInstanceDynamic)))))))