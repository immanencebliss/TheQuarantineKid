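; Base actor for render surfaces, showing a scene capture on a static mesh through a render target.
; Enabling rendering creates the render target, optionally viewport-sized, and feeds it from the SceneCaptureComponent2D into a dynamic material on the mesh.
; Helpers match the capture's FOV to the player camera and decide whether updates are needed, using optional distance and facing-direction visibility checks.
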(fn ConstructionScript
  (Components|StaticMesh|SetStaticMesh (Variables|Default|GetStaticMesh) (Variables|Mesh|GetRenderMeshAsset)))

(fn InitSceneCapture
  (if (Variables|Capture|GetbRT_UseViewportSize)
    (Variables|Capture|SetRT_Resolution (Viewport|GetViewportSize)))
  (bind _returnvalue (Rendering|CreateRenderTarget2D (Math|Float|Truncate (.x (Variables|Capture|GetRT_Resolution))) (Math|Float|Truncate (.y (Variables|Capture|GetRT_Resolution))) (Variables|Capture|GetRT_Format)))
  (bind _output_get (Variables|Default|SetRenderTarget _returnvalue))
  (Variables|/Script/Engine.SceneCaptureComponent2D|SetTextureTarget (Variables|Default|GetSceneCaptureComponent2D) _output_get)
  (bind _returnvalue_2 (Rendering|Material|CreateDynamicMaterialInstance (Variables|Mesh|GetRenderMaterialAsset) "None" :!class /Script/Engine.KismetMaterialLibrary))
  (Variables|Default|SetMID _returnvalue_2)
  (Rendering|Material|SetTextureParameterValue (Variables|Default|GetMID) "TextureRT" (Variables|Default|GetRenderTarget))
  (Rendering|Material|SetMaterial (Variables|Default|GetStaticMesh) 0 (Variables|Default|GetMID)))

(fn CheckSCCNeedstoUpdate
  (if (Variables|Capture|GetbUseUpdateDistance)
    (bind _visible (CallFunction|CheckVisibilitybyDistance (Variables|Capture|GetMaxRenderUpdateDistance) (Transformation|GetActorLocation))))
  (if (Variables|Capture|GetbUseUpdateDirection)
    (bind _visible_2 (CallFunction|CheckVisibilitybyDirection (Transformation|GetActorLocation) (Transformation|GetActorForwardVector))))
  (return (select (Variables|Capture|GetbUseUpdateDirection) (and _visible_2 (select (Variables|Capture|GetbUseUpdateDistance) _visible true)) (select (Variables|Capture|GetbUseUpdateDistance) _visible true))))

(fn EnableRender
  (Variables|Capture|SetbRenderEnabled true)
  (CallFunction|InitSceneCapture))

(fn UpdateSCC2DTransform
  (Variables|/Script/Engine.SceneCaptureComponent2D|SetFOVAngle (Variables|Default|GetSceneCaptureComponent2D) (Camera|GetFOVAngle (Game|GetPlayerCameraManager 0))))