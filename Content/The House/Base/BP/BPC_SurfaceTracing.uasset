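; Surface-tracing component that fires debug-drawn line traces that ricochet or pass through portals to push physics actors.
; TraceLoop mirrors the direction at each hit, spending remaining distance across bounces.
; TracePortal traces once, its ricochet loop unwired, remaps portal hits via TracePortalRecursive, then applies the player's STImpulse to any BP_PhysActor found.
; TracePortalRecursive follows chained portals but discards nested results, returning its own hit.
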(fn TraceLoop
  (params (TraceStart :type Vector) (TraceDirection :type Vector) (TraceDistance :type Float%20%28single-precision%29) (NumRicochets :type Integer))
  (LocalVariables|SetLocalTraceStart TraceStart)
  (LocalVariables|SetLocalTraceDirection (Math|Vector|Normalize TraceDirection))
  (LocalVariables|SetLocalTraceDistance TraceDistance)
  (LocalVariables|SetLocalTraceEnd (+ (LocalVariables|GetLocalTraceStart) (* (LocalVariables|GetLocalTraceDirection) (LocalVariables|GetLocalTraceDistance))))
  (for _index (range 0 NumRicochets)
    (bind (_outhit _returnvalue) (Collision|LineTraceByChannel (LocalVariables|GetLocalTraceStart) (LocalVariables|GetLocalTraceEnd) "TraceTypeQuery1" false 0 "ForDuration"))
    (if _returnvalue
      (LocalVariables|SetLocalTraceImpactPoint (.ImpactPoint (Collision|BreakHitResult _outhit)))
      (LocalVariables|SetLocalTraceImpactNormal (.ImpactNormal (Collision|BreakHitResult _outhit)))
      (LocalVariables|SetLocalTraceDistance (- (LocalVariables|GetLocalTraceDistance) (.Distance (Collision|BreakHitResult _outhit))))
      ;[1 1 1] Next trace params
      (LocalVariables|SetLocalTraceDirection (Math|Vector|MirrorVectorbyNormal (LocalVariables|GetLocalTraceDirection) (LocalVariables|GetLocalTraceImpactNormal)))
      (LocalVariables|SetLocalTraceStart (+ (LocalVariables|GetLocalTraceImpactPoint) (LocalVariables|GetLocalTraceDirection)))
      (LocalVariables|SetLocalTraceEnd (+ (LocalVariables|GetLocalTraceStart) (* (LocalVariables|GetLocalTraceDirection) (LocalVariables|GetLocalTraceDistance))))
      ;[1 1 1] Debug
      (CallFunction|DrawDebugGizmo (LocalVariables|GetLocalTraceImpactPoint) (Math|Rotator|MakeRotfromXZ (Math|Vector|CrossProduct (Math|Vector|CrossProduct (Math|Vector|NegateVector (LocalVariables|GetLocalTraceDirection)) (LocalVariables|GetLocalTraceImpactNormal)) (LocalVariables|GetLocalTraceImpactNormal)) (LocalVariables|GetLocalTraceImpactNormal)) 5.0)
      (Rendering|Debug|DrawDebugString (LocalVariables|GetLocalTraceImpactPoint) (Utilities|String|ToString(Integer) _index) 0 "(R=1.000000,G=1.000000,B=1.000000,A=1.000000)" 5.0))))

(fn TracePortal
  (params (TraceStart :type Vector) (TraceDirection :type Vector) (TraceDistance :type Float%20%28single-precision%29) (NumRicochets :type Integer))
  (LocalVariables|SetLocalTraceStart TraceStart)
  (LocalVariables|SetLocalTraceDirection (Math|Vector|Normalize TraceDirection))
  (LocalVariables|SetLocalTraceDistance TraceDistance)
  (LocalVariables|SetLocalTraceEnd (+ (LocalVariables|GetLocalTraceStart) (* (LocalVariables|GetLocalTraceDirection) (LocalVariables|GetLocalTraceDistance))))
  (bind (_outhit _returnvalue) (Collision|LineTraceByChannel (LocalVariables|GetLocalTraceStart) (LocalVariables|GetLocalTraceEnd) "TraceTypeQuery1" false 0 "ForDuration"))
  (if _returnvalue
    (LocalVariables|SetLocalTraceImpactPoint (.ImpactPoint (Collision|BreakHitResult _outhit)))
    (LocalVariables|SetLocalTraceImpactNormal (.ImpactNormal (Collision|BreakHitResult _outhit)))
    (LocalVariables|SetLocalHitActor (.HitActor (Collision|BreakHitResult _outhit)))
    (LocalVariables|SetLocalTraceDistance (- (LocalVariables|GetLocalTraceDistance) (.Distance (Collision|BreakHitResult _outhit))))
    (bind _asbp_portal (Utilities|Casting|CastToBP_Portal (LocalVariables|GetLocalHitActor))
      (:then
        (bind (_tracedirection _traceimpactpoint _traceimpactnormal _hitactor) (CallFunction|TracePortalRecursive _asbp_portal (LocalVariables|GetLocalTraceDirection) (LocalVariables|GetLocalTraceDistance) (LocalVariables|GetLocalTraceImpactPoint)))
        (LocalVariables|SetLocalTraceDirection _tracedirection)
        (LocalVariables|SetLocalTraceImpactPoint _traceimpactpoint)
        (LocalVariables|SetLocalTraceImpactNormal _traceimpactnormal)
        (LocalVariables|SetLocalHitActor _hitactor))
      (:CastFailed
        _))
    ;[1 1 1] Push PhysActor with specified impulse
    (bind _asbp_phys_actor (Utilities|Casting|CastToBP_PhysActor (LocalVariables|GetLocalHitActor))
      (:then
        (bind _asbp_first_person_character (Utilities|Casting|CastToBP_FirstPersonCharacter (Game|GetPlayerCharacter 0)))
        (CallFunction|PushPhysActor _asbp_phys_actor (LocalVariables|GetLocalTraceDirection) (Variables|/Game/GameMode/FirstPerson/BP_FirstPersonCharacter.BP_FirstPersonCharacter_C|GetST_Impulse _asbp_first_person_character)))
      (:CastFailed
        ;[1 1 1] Next trace params
        (LocalVariables|SetLocalTraceDirection (Math|Vector|MirrorVectorbyNormal (LocalVariables|GetLocalTraceDirection) (LocalVariables|GetLocalTraceImpactNormal)))
        (LocalVariables|SetLocalTraceStart (+ (LocalVariables|GetLocalTraceImpactPoint) (LocalVariables|GetLocalTraceDirection)))
        (LocalVariables|SetLocalTraceEnd (+ (LocalVariables|GetLocalTraceStart) (* (LocalVariables|GetLocalTraceDirection) (LocalVariables|GetLocalTraceDistance))))
        ;[1 1 1] Debug
        (CallFunction|DrawDebugGizmo (LocalVariables|GetLocalTraceImpactPoint) (Math|Rotator|MakeRotfromXZ (Math|Vector|CrossProduct (Math|Vector|CrossProduct (Math|Vector|NegateVector (LocalVariables|GetLocalTraceDirection)) (LocalVariables|GetLocalTraceImpactNormal)) (LocalVariables|GetLocalTraceImpactNormal)) (LocalVariables|GetLocalTraceImpactNormal)) 2e+01)
        (Rendering|Debug|DrawDebugString (LocalVariables|GetLocalTraceImpactPoint) (Utilities|String|ToString(Integer) (stale _index)) 0 "(R=1.000000,G=1.000000,B=1.000000,A=1.000000)" 2e+01)))))

(fn TracePortalRecursive
  (params (PortalActor :type BP%20Portal%20Object%20Reference) (PreviousTraceDirection :type Vector) (TraceDistance :type Float%20%28single-precision%29) (PreviousImpactPoint :type Vector))
  (LocalVariables|SetLocalPortalActor PortalActor)
  (bind _newdirection (CallFunction|PortalConvertDirection (LocalVariables|GetLocalPortalActor) (Variables|/Game/Portals/BP_Portal.BP_Portal_C|GetTargetPortal (LocalVariables|GetLocalPortalActor)) PreviousTraceDirection))
  (LocalVariables|SetNewTraceDirection _newdirection)
  (bind _newlocation (CallFunction|PortalConvertLocation (LocalVariables|GetLocalPortalActor) (Variables|/Game/Portals/BP_Portal.BP_Portal_C|GetTargetPortal (LocalVariables|GetLocalPortalActor)) PreviousImpactPoint))
  (LocalVariables|SetNewTraceStart _newlocation)
  (LocalVariables|SetLocalTraceDistance TraceDistance)
  (LocalVariables|SetNewTraceEnd (+ (LocalVariables|GetNewTraceStart) (* (LocalVariables|GetNewTraceDirection) (LocalVariables|GetLocalTraceDistance))))
  (bind (_outhit _returnvalue) (Collision|LineTraceByChannel (LocalVariables|GetNewTraceStart) (LocalVariables|GetNewTraceEnd) "TraceTypeQuery1" false 0 "ForDuration"))
  (if _returnvalue
    (LocalVariables|SetLocalImpactPoint (.ImpactPoint (Collision|BreakHitResult _outhit)))
    (LocalVariables|SetLocalImpactNormal (.ImpactNormal (Collision|BreakHitResult _outhit)))
    (LocalVariables|SetLocalHitActor (.HitActor (Collision|BreakHitResult _outhit)))
    (bind _asbp_portal (Utilities|Casting|CastToBP_Portal (LocalVariables|GetLocalHitActor))
      (:then
        (CallFunction|TracePortalRecursive _asbp_portal (LocalVariables|GetNewTraceDirection) (- (LocalVariables|GetLocalTraceDistance) (.Distance (Collision|BreakHitResult _outhit))) (LocalVariables|GetLocalImpactPoint)))
      (:CastFailed
        _))
    (return (LocalVariables|GetNewTraceDirection) (LocalVariables|GetLocalImpactPoint) (LocalVariables|GetLocalImpactNormal) (LocalVariables|GetLocalHitActor))))

(fn PushPhysActor
  (params (PhysActor :type BP%20Phys%20Actor%20Object%20Reference) (Direction :type Vector) (Impulse :type Float%20%28single-precision%29))
  (Physics|AddImpulse (Variables|/Game/Physics/BP_PhysActor.BP_PhysActor_C|GetStaticMesh PhysActor) (* Direction Impulse) "None" true))