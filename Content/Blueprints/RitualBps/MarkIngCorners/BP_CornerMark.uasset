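; BP_CornerMark is a ritual corner mark that displays one of four word symbols on a plane with a dissolve effect.
; The construction script creates a dynamic material instance for the plane.
; SetMatieral maps the given word to a symbol texture, makes the plane visible and triggers the dissolve.
; A timeline drives the material's dissolve parameter, and also plays on BeginPlay.
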(event Custom|Dissolve%20In%20Texture
  (bind _dissolveintexture (Timeline|DissolveInTexture Play)
    (:Update
      (Rendering|Material|SetScalarParameterValue (Variables|Default|GetCornerTexture) "disolve" (Math|Float|Lerp 0.0 1.0 _dissolveintexture) :!class /Script/Engine.MaterialInstanceDynamic))))

(event EventBeginPlay
  (CallFunction|DissolveinTexture))

(event Collision|EventActorBeginOverlap
  (params (OtherActor :type Actor%20Object%20Reference)))

(event EventTick
  (params (DeltaSeconds :type Float%20%28single-precision%29)))

(fn ConstructionScript
  (bind _returnvalue (Rendering|Material|CreateDynamicMaterialInstance (Variables|Default|GetPlane) 0 "/Game/Blueprints/RitualBps/MarkIngCorners/MAT_CornerMark_Inst.MAT_CornerMark_Inst" "None" :!class /Script/Engine.PrimitiveComponent))
  (Variables|Default|SetCornerTexture _returnvalue))

(fn SetMatieral
  (params (word :type String))
  (switch string word
    (:rebirth
      (Rendering|Material|SetTextureParameterValue (Variables|Default|GetCornerTexture) "symbol" "/Game/Blueprints/RitualBps/MarkIngCorners/WordOfPower/Rebirth.Rebirth"))
    (:innocence
      (Rendering|Material|SetTextureParameterValue (Variables|Default|GetCornerTexture) "symbol" "/Game/Blueprints/RitualBps/MarkIngCorners/WordOfPower/Innocence.Innocence"))
    (:ethereal
      (Rendering|Material|SetTextureParameterValue (Variables|Default|GetCornerTexture) "symbol" "/Game/Blueprints/RitualBps/MarkIngCorners/WordOfPower/ethereal.ethereal"))
    (:absolution
      (Rendering|Material|SetTextureParameterValue (Variables|Default|GetCornerTexture) "symbol" "/Game/Blueprints/RitualBps/MarkIngCorners/WordOfPower/Absolution.Absolution")))
  (Rendering|SetVisibility (Variables|Default|GetPlane) true false)
  (CallFunction|DissolveinTexture))