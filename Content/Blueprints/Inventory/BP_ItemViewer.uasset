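; BP_ItemViewer is an inventory item preview that shows an item's static mesh and spins it continuously.
; UpdateViewer offsets the mesh, sets CurrentItem to None, then reads that same variable for relative distance, elevation and mesh.
; Tick adds a local rotation of Speed each frame, without delta-time scaling, so spin rate follows frame rate.
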(event Custom|UpdateViewer
  (Transformation|AddLocalOffset (Variables|Default|GetStaticMesh) (Math|Vector|MakeVector (Variables|Default|GetCurrentItemDistance) 0.0 (Variables|Default|GetCurrentItemElevation)) false false)
  (bind _output_get (Variables|Default|SetCurrentItem ""))
  (Transformation|SetRelativeLocation (Variables|Default|GetStaticMesh) (Math|Vector|MakeVector (.itemdistance _output_get) 0.0 (.itemelevation _output_get)) false false)
  (Components|StaticMesh|SetStaticMesh (Variables|Default|GetStaticMesh) (.mesh _output_get)))

(event EventTick
  (params (DeltaSeconds :type Float%20%28single-precision%29))
  (Transformation|AddLocalRotation (Variables|Default|GetStaticMesh) (Variables|Default|GetSpeed) false false))

(fn ConstructionScript)