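; BP_SpawnManager is an AI wave spawner manager that keeps adding enemies until a maximum count is reached.
; Tick passes through a DoOnce gate, increments the enemy count and calls SpawnEnemy on a random entry in its Spawners array.
; The gate reopens through ResetRespawn after the SpawnRate delay, or immediately when at the cap, so it keeps checking for free slots.
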(event Custom|ResetRespawn
  (bind _spawners (Variables|Default|GetSpawners))
  (Utilities|FlowControl|DoOnce false) ; enters at Reset
)

(event EventBeginPlay)

(event Collision|EventActorBeginOverlap
  (params (OtherActor :type Actor%20Object%20Reference)))

(event EventTick
  (params (DeltaSeconds :type Float%20%28single-precision%29))
  (bind _spawners (Variables|Default|GetSpawners))
  (Utilities|FlowControl|DoOnce false
    (:Completed
      (if (< (Variables|Default|GetAmountOfEnemies) (Variables|Default|GetMaXEnemies))
        (Math|Integer|IncrementInt (Variables|Default|GetAmountOfEnemies)
          (:%20%20
            (Default|SpawnEnemy (Utilities|Array|Get(acopy) _spawners (Math|Random|RandomIntegerinRange 0 (- (Utilities|Array|Length _spawners) 1))))
            (Utilities|FlowControl|Delay (Variables|Default|GetSpawnRate))
            (CallFunction|ResetRespawn)))
        (else
          (CallFunction|ResetRespawn))))))

(fn ConstructionScript)