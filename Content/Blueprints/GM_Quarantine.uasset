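; GM_Quarantine is a game mode Blueprint that drives a day/night cycle and hands queued packages over at nightfall.
; A looping 180-second timer started on BeginPlay drives a FlipFlop that alternates day and night start events, firing day first.
; Night start appends TomorrowsPackage to TodaysPackage and prints a debug count, while day start is empty.
; The node that clears TomorrowsPackage is disconnected, so its entries are appended again each night.
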(event Custom|OnDayStart)

(event Custom|OnNightStart
  (bind _tomorrowspackage (Variables|Default|GetTomorrowsPackage))
  (for _array_element _tomorrowspackage
    (Utilities|Array|Add (Variables|Default|GetTodaysPackage) _array_element))
  (Development|PrintString (Utilities|String|Append "night mode package lenght " (Utilities|String|ToString(Integer) (Utilities|Array|Length _tomorrowspackage)))))

(event Custom|Cycle
  (Utilities|FlowControl|FlipFlop
    (:A
      (CallFunction|OnDayStart))
    (:B
      (CallFunction|OnNightStart))))

(event EventBeginPlay
  (bind _returnvalue (Utilities|Time|SetTimerbyEvent (delegate Custom|Cycle) 1.8e+02 true))
  (Variables|Default|SetDayNightTimer _returnvalue))

(fn ConstructionScript)