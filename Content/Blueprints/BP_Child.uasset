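; Child (baby) actor with survival needs that the first-person player picks up or puts down through Interact, toggling the baby's visibility.
; Looping one-second timers update clamped Hunger, Cold and Restlessness, with restlessness rate set by sleep state on Tick.
; Each need maps to a tiered modifier added to Trauma's rate, gated by 25-second timers.
; As written, all three delayed updates write only HungerModifier from LastHungerModifier.
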(event Custom|RestlessnessTimer
  ;[1 1 1] Fatigue
  (bind _returnvalue (Utilities|Time|SetTimerbyEvent (delegate Custom|IncreaseRestlessnessOverTime) 1.0 true))
  (Variables|Timers|SetRestlessnessHandle _returnvalue))

(event Custom|IncreaseRestlessnessOverTime
  ;[1 1 1] Fatigue
  (CallFunction|IncreaseRestlessness (Variables|Default|GetRestlessness%20Rate))
  (bind _modifier (CallFunction|TraumaCalculation (Variables|Stats|GetRestlessness)))
  (bind _output_get (Variables|Modifiers|SetPendingRestlessnessModifier _modifier))
  (if (Variables|Modifiers|GetCanUpdateLRM)
    (bind _output_get_2 (Variables|Modifiers|SetLastRestlessnessModifier _output_get))
    (if (== _output_get_2 (Variables|Modifiers|GetRestlessnessModifier))
      (goto _label Reset)
      (else
        _))
    (else
      (bind _canupdate (CallFunction|ClearTimer (Variables|Modifiers|GetPendingRestlessnessModifier) (Variables|Modifiers|GetLastRestlessnessModifier)))
      (bind _output_get_3 (Variables|Modifiers|SetCanUpdateLRM _canupdate))
      (if _output_get_3
        _
        (else
          (goto _label Reset)))))
  (Utilities|FlowControl|DoOnce false :!label _label
    (:Completed
      (Variables|Modifiers|SetCanUpdateLRM false)
      (CallFunction|RestlessnessTime))))

(event Custom|TraumaTimer
  ;[1 1 1] Trauma
  (bind _returnvalue (Utilities|Time|SetTimerbyEvent (delegate Custom|IncreaseTraumaOverTime) 1.0 true))
  (Variables|Timers|SetTraumaHandle _returnvalue))

(event Custom|IncreaseTraumaOverTime
  ;[1 1 1] Trauma
  (bind _output_get (Variables|Default|SetModifiedTraumRate (+ (Variables|Default|GetTraumaRate) (Variables|Modifiers|GetHungerModifier) (Variables|Modifiers|GetColdModifier) (Variables|Modifiers|GetRestlessnessModifier))))
  (CallFunction|TraumaController _output_get))

(event Custom|RestlessnessTime
  ;[1 1 1] Fatigue
  (Utilities|Time|ClearandInvalidateTimerbyHandle (Variables|Timers|GetRestlessnessTimeHandle))
  (bind _returnvalue (Utilities|Time|SetTimerbyEvent (delegate Custom|IncrementRestlessnessModifier) 25.0))
  (Variables|Timers|SetRestlessnessTimeHandle _returnvalue))

(event Custom|IncrementRestlessnessModifier
  ;[1 1 1] Fatigue
  (Variables|Modifiers|SetHungerModifier (Variables|Modifiers|GetLastHungerModifier))
  (Variables|Modifiers|SetCanUpdateLRM true))

(event Custom|HungerTime
  ;[1 1 1] Hunger
  (Utilities|Time|ClearandInvalidateTimerbyHandle (Variables|Timers|GetHungerTimeHandle))
  (bind _returnvalue (Utilities|Time|SetTimerbyEvent (delegate Custom|IncrementHungerModifier) 25.0))
  (Variables|Timers|SetHungerTimeHandle _returnvalue))

(event Custom|IncrementHungerModifier
  ;[1 1 1] Hunger
  (Variables|Modifiers|SetHungerModifier (Variables|Modifiers|GetLastHungerModifier))
  (Variables|Modifiers|SetCanUpdateLHM true))

(event Custom|ColdTime
  ;[1 1 1] Cold
  (Utilities|Time|ClearandInvalidateTimerbyHandle (Variables|Timers|GetColdTimeHandle))
  (bind _returnvalue (Utilities|Time|SetTimerbyEvent (delegate Custom|IncrementColdModifier) 25.0))
  (Variables|Timers|SetColdTimeHandle _returnvalue))

(event Custom|IncrementColdModifier
  ;[1 1 1] Cold
  (Variables|Modifiers|SetHungerModifier (Variables|Modifiers|GetLastHungerModifier))
  (Variables|Modifiers|SetCanUpdateLCM true))

(event Custom|HungerTimer
  ;[1 1 1] Hunger
  (bind _returnvalue (Utilities|Time|SetTimerbyEvent (delegate Custom|IncreaseHungerOverTime) 1.0 true))
  (Variables|Timers|SetHungerHandle _returnvalue))

(event Custom|IncreaseHungerOverTime
  ;[1 1 1] Hunger
  (CallFunction|IncreaseHunger 0.6)
  (bind _modifier (CallFunction|TraumaCalculation (Variables|Stats|GetHunger)))
  (bind _output_get (Variables|Modifiers|SetPendingHungerModifier _modifier))
  (if (Variables|Modifiers|GetCanUpdateLHM)
    (bind _output_get_2 (Variables|Modifiers|SetLastHungerModifier _output_get))
    (if (== _output_get_2 (Variables|Modifiers|GetHungerModifier))
      (goto _label Reset)
      (else
        _))
    (else
      (bind _canupdate (CallFunction|ClearTimer (Variables|Modifiers|GetPendingHungerModifier) (Variables|Modifiers|GetLastHungerModifier)))
      (bind _output_get_3 (Variables|Modifiers|SetCanUpdateLHM _canupdate))
      (if _output_get_3
        _
        (else
          (goto _label Reset)))))
  (Utilities|FlowControl|DoOnce false :!label _label
    (:Completed
      (Variables|Modifiers|SetCanUpdateLHM false)
      (CallFunction|HungerTime))))

(event Custom|ColdTimer
  ;[1 1 1] Cold
  (bind _returnvalue (Utilities|Time|SetTimerbyEvent (delegate Custom|IncreaseColdOVerTime) 1.0 true))
  (Variables|Timers|SetColdHandle _returnvalue))

(event Custom|IncreaseColdOVerTime
  ;[1 1 1] Cold
  (CallFunction|IncreaseCold (Variables|Default|GetColdRate))
  (bind _modifier (CallFunction|TraumaCalculation (Variables|Stats|GetCold)))
  (bind _output_get (Variables|Modifiers|SetPendingColdModifier _modifier))
  (if (Variables|Modifiers|GetCanUpdateLCM)
    (bind _output_get_2 (Variables|Modifiers|SetLastColdModifier _output_get))
    (if (== _output_get_2 (Variables|Modifiers|GetColdModifier))
      (goto _label Reset)
      (else
        _))
    (else
      (bind _canupdate (CallFunction|ClearTimer (Variables|Modifiers|GetPendingColdModifier) (Variables|Modifiers|GetLastColdModifier)))
      (bind _output_get_3 (Variables|Modifiers|SetCanUpdateLCM _canupdate))
      (if _output_get_3
        _
        (else
          (goto _label Reset)))))
  (Utilities|FlowControl|DoOnce false :!label _label
    (:Completed
      (Variables|Modifiers|SetCanUpdateLCM false)
      (CallFunction|ColdTime))))

(event EventBeginPlay
  ;[1 1 1] Event Begin Play
  (Utilities|FlowControl|Sequence
    (:then_0
      (CallFunction|HungerTimer))
    (:then_1
      (CallFunction|ColdTimer))
    (:then_2
      (CallFunction|RestlessnessTimer))
    (:then_3
      (CallFunction|TraumaTimer))))

(event EventInteract
  (params (HitComponent :type Actor%20Component%20Object%20Reference))
  (bind _baby (Variables|Default|GetBaby))
  ;[1 1 1] Event Interact
  (bind _asfirst_person_character (Utilities|Casting|CastToFirstPersonCharacter (Game|GetPlayerCharacter 0)))
  (bind _output_get (Variables|Default|SetPlayer _asfirst_person_character))
  (if (Variables|/Game/FirstPersonBP/Blueprints/FirstPersonCharacter.FirstPersonCharacter_C|GetHasBaby _output_get)
    (Rendering|SetVisibility _baby true false)
    (Default|HoldChild (Variables|Default|GetPlayer) :!label _label)
    (elif (Variables|Default|GetBabyHere)
      (Rendering|SetVisibility _baby false false)
      (goto _label))))

(event EventTick
  (params (DeltaSeconds :type Float%20%28single-precision%29))
  ;[1 1 1] Event Tick
  (CallFunction|SetBaseRestlessnessRate))

(fn ConstructionScript)

(fn IncreaseHunger
  (params (Rate :type Float%20%28single-precision%29))
  (Variables|Stats|SetHunger (Math|Float|Clamp(Float) (+ (Variables|Stats|GetHunger) Rate) 0.0 1e+02)))

(fn IncreaseCold
  (params (Rate :type Float%20%28single-precision%29))
  (Variables|Stats|SetCold (Math|Float|Clamp(Float) (+ (Variables|Stats|GetCold) Rate) 0.0 1e+02)))

(fn IncreaseRestlessness
  (params (Rate :type Float%20%28single-precision%29))
  (Variables|Stats|SetRestlessness (Math|Float|Clamp(Float) (+ (Variables|Stats|GetRestlessness) Rate) 0.0 1e+02)))

(fn SetBaseRestlessnessRate
  (if (Variables|Default|GetIsAsleep)
    (Variables|Default|SetRestlessness%20Rate 0.5)
    (else
      (Variables|Default|SetRestlessness%20Rate -0.5))))

(fn TraumaController
  (params (B :type Float%20%28single-precision%29))
  (Variables|Stats|SetTrauma (Math|Float|Clamp(Float) (+ (Variables|Stats|GetTrauma) B) 0.0 2e+02)))

(fn TraumaCalculation
  (params (Stat :type Float%20%28single-precision%29))
  (if (Math|Float|InRange(Float) Stat 0.0 25.0)
    (LocalVariables|SetMod 0.0)
    (return (LocalVariables|GetMod))
    (elif (Math|Float|InRange(Float) Stat 25.0 5e+01 false)
      (LocalVariables|SetMod 0.1)
      (return (LocalVariables|GetMod))
      (elif (Math|Float|InRange(Float) Stat 5e+01 75.0 false)
        (LocalVariables|SetMod 0.2)
        (return (LocalVariables|GetMod))
        (elif (Math|Float|InRange(Float) Stat 75.0 1e+02 false)
          (LocalVariables|SetMod 0.3)
          (return (LocalVariables|GetMod)))))))

(fn ClearTimer
  (params (Pending%20Mod :type Float%20%28single-precision%29) (LastMod :type Float%20%28single-precision%29))
  (if (not (== Pending%20Mod LastMod))
    (if (> LastMod 0.0)
      (if (> Pending%20Mod LastMod)
        (LocalVariables|SetCan%20Update? false :!label _label)
        (else
          (LocalVariables|SetCan%20Update? false :!label _label_2)))
      (elif (< LastMod 0.0)
        (if (< Pending%20Mod LastMod)
          (goto _label)
          (else
            (goto _label_2)))
        (else
          (goto _label_2))))
    (return (LocalVariables|GetCan%20Update?))))