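; Baby is an interactable Blueprint that runs a scripted finale scare when the Interact event fires.
; The construction script creates a dynamic material instance on its static mesh for a later texture swap.
; Interact blends the player's view to a camera and plays the Finale level sequence.
; Timed delays then slam a door, trigger a short light flicker and switch the baby's texture to a corrupted version.
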(event EventInteract
  (params (HitComponent :type Actor%20Component%20Object%20Reference))
  (Game|Player|SetViewTargetwithBlend (Game|GetPlayerController 0) (Variables|Default|GetCamera) 1.0 "VTBlend_Linear" 0.0 false)
  (Utilities|FlowControl|Delay 1.0)
  (bind _returnvalue (Sequencer|Player|CreateLevelSequencePlayer "/Game/Finale.Finale"))
  (Sequencer|Player|Play _returnvalue :!class /Script/MovieScene.MovieSceneSequencePlayer)
  (Utilities|FlowControl|Delay 13.0)
  (Default|SlamDoor (Variables|Default|GetDoor))
  (Utilities|FlowControl|Delay 1.0)
  (Default|IFlickerShort (Variables|Default|GetLight) false)
  (Utilities|FlowControl|Delay 3.5)
  (Rendering|Material|SetTextureParameterValue (Variables|Default|GetMatInst) "Texture" "/Game/ThirdPersonBP/BabyCorrupted.BabyCorrupted"))

(fn ConstructionScript
  (bind _staticmesh (Variables|Default|GetStaticMesh))
  (|CallParentFunction)
  (bind _returnvalue (Rendering|Material|CreateDynamicMaterialInstance _staticmesh 0 (Rendering|Material|GetMaterial _staticmesh 0) "None" :!class /Script/Engine.PrimitiveComponent))
  (Variables|Default|SetMatInst _returnvalue))