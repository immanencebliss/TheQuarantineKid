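; Placeable is a Blueprint for objects placed in the game, supplying a temporary "building" look and a way to undo it.
; SaveMaterialAndSetToBlue maps a dynamic instance of every static mesh material to its mesh and slot, then applies the Building material.
; RestoreAll reapplies those saved instances from the MatMesh map.
; OnPlaceComplete is an empty stub, and the event graph runs no logic.
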(event EventBeginPlay)

(event Collision|EventActorBeginOverlap
  (params (OtherActor :type Actor%20Object%20Reference)))

(event EventTick
  (params (DeltaSeconds :type Float%20%28single-precision%29)))

(fn ConstructionScript)

(fn OnPlaceComplete)

(fn SaveMaterialandSettoBlue
  (Utilities|Map|Clear (Variables|Default|GetMatMesh))
  (for _array_element (Actor|GetComponentsByClass "/Script/Engine.StaticMeshComponent")
    (for (_array_element_2 _array_index) (Rendering|Material|GetMaterials _array_element)
      (bind _returnvalue (Rendering|Material|CreateDynamicMaterialInstance _array_element_2 "None" :!class /Script/Engine.KismetMaterialLibrary))
      (Utilities|Map|Add (Variables|Default|GetMatMesh) _returnvalue (Utilities|Struct|MakeMeshAndMaterial _array_element _array_index))
      (Rendering|Material|SetMaterial _array_element _array_index "/Game/Art/building.building"))))

(fn RestoreAll
  (bind _keys (Utilities|Map|Keys (Variables|Default|GetMatMesh)))
  (for _array_element _keys
    (Rendering|Material|SetMaterial (.meshes (Utilities|Struct|BreakMeshAndMaterial (.Value (Utilities|Map|Find (Variables|Default|GetMatMesh) _array_element)))) (.index (Utilities|Struct|BreakMeshAndMaterial (.Value (Utilities|Map|Find (Variables|Default|GetMatMesh) _array_element)))) _array_element)))