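; Corpse cart actor for the Pier that displays up to three bodies as separate mesh components, starting full at BeginPlay.
; UpdateBodyCount stores the count, then uses two cascading switches to hide meshes above it and show those within it.
; A SetActivity helper toggles each mesh's visibility and collision together, so hidden bodies do not block.
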(event EventBeginPlay
  (CallFunction|UpdateBodyCount 3))

(event Collision|EventActorBeginOverlap
  (params (OtherActor :type Actor%20Object%20Reference)))

(event EventTick
  (params (DeltaSeconds :type Float%20%28single-precision%29)))

(fn ConstructionScript)

(fn UpdateBodyCount
  (params (newCount :type Integer))
  (bind _output_get (Variables|Default|SetbodyCount newCount))
  (switch int _output_get
    (:Default
      (Utilities|SetActivity (Variables|Default|GetcorpseCartV2_Roundcube_004) false :!label _label)
      (Utilities|SetActivity (Variables|Default|GetcorpseCartV2_Roundcube_005) false :!label _label_2)
      (Utilities|SetActivity (Variables|Default|GetcorpseCartV2_Roundcube_006) false :!label _label_3))
    (:0
      (goto _label))
    (:1
      (goto _label_2))
    (:2
      (goto _label_3))
    (:3
      _))
  (switch int (Variables|Default|GetbodyCount)
    (:1
      _)
    (:2
      (Utilities|SetActivity (Variables|Default|GetcorpseCartV2_Roundcube_005) true :!label _label_4))
    (:3
      (Utilities|SetActivity (Variables|Default|GetcorpseCartV2_Roundcube_006) true)
      (goto _label_4)))
  (Utilities|SetActivity (Variables|Default|GetcorpseCartV2_Roundcube_004) true))