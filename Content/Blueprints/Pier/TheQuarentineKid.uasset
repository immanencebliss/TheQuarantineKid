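; The Quarentine Kid is a Pier Blueprint for a kid whose mesh animation depends on whether it has been caught.
; Every Tick calls the parent Tick, then runs ChildCaught to poll the IsCaught flag.
; ChildCaught plays the mesh animation at normal rate while the flag is true and freezes it at zero rate otherwise.
; Nothing in this graph sets IsCaught.
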(event EventBeginPlay
  (|CallParentFunction) ; This node is disabled and will not be called.\nDrag off pins to build functionality.
)

(event Collision|EventActorBeginOverlap
  (params (OtherActor :type Actor%20Object%20Reference))
  (|CallParentFunction OtherActor) ; This node is disabled and will not be called.\nDrag off pins to build functionality.
)

(event EventTick
  (params (DeltaSeconds :type Float%20%28single-precision%29))
  (|CallParentFunction DeltaSeconds)
  (CallFunction|ChildCaught))

(fn ConstructionScript
  (|CallParentFunction))

(fn ChildCaught
  (if (Variables|Default|GetisCaught)
    (Components|Timeline|SetPlayRate (Variables|Character|GetMesh) 1.0)
    (else
      (Components|Timeline|SetPlayRate (Variables|Character|GetMesh) 0.0))))