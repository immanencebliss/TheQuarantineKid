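; Front door actor for the residential house that opens and closes through its animation Blueprint.
; BeginPlay caches the DoorMain mesh's AnimBPDoorMain instance, whose PlayerNear flag drives the door state.
; Force clears the flag to close and ForceClosed sets it to open, opposite to what the latter's name suggests.
; The trigger's end-overlap event is empty, and a toggle branch on the flag is never run.
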(event OnComponentEndOverlap(Trigger)
  (params (OverlappedComponent :type Primitive%20Component%20Object%20Reference) (OtherActor :type Actor%20Object%20Reference) (OtherComp :type Primitive%20Component%20Object%20Reference) (OtherBodyIndex :type Integer)))

(event Custom|Force
  ;[1 1 1] Open and closes door when player interacts with it
  ;;[1 1 1] Close Door
  (Variables|/Game/HQ_ResidentialHouse/Meshes/DoorMain/AnimBPDoorMain.AnimBPDoorMain_C|SetPlayerNear (Variables|Default|GetCastToDoorAnim) false))

(event Custom|Force%20Closed
  ;[1 1 1] Open and closes door when player interacts with it
  ;;[1 1 1] Open Door
  (Variables|/Game/HQ_ResidentialHouse/Meshes/DoorMain/AnimBPDoorMain.AnimBPDoorMain_C|SetPlayerNear (Variables|Default|GetCastToDoorAnim) true))

(event EventBeginPlay
  (bind _asanim_bpdoor_main (Utilities|Casting|CastToAnimBPDoorMain (Components|SkeletalMesh|GetAnimInstance (Variables|Default|GetDoor_main))))
  (Variables|Default|SetCastToDoorAnim _asanim_bpdoor_main))

(fn ConstructionScript)